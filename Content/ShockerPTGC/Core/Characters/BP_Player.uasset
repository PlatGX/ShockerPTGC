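; BP_Player is the player character that slides a Paddle component horizontally and handles pausing.
; It adds the default Enhanced Input mapping context when its controller changes.
; Move input is scaled and added to the paddle's world X, clamped to fixed bounds.
; A pause widget created at BeginPlay is toggled by a FlipFlop on the pause input, along with the game's paused state.
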(event `self.ReceiveControllerChanged`
  (params (OldController :type "Controller Object Reference") (NewController :type "Controller Object Reference"))
  (bind _asplayer_controller (cast `PlayerController` NewController))
  (`EnhancedInputSubsystemInterface.AddMappingContext` (pcsubsystem `EnhancedInputLocalPlayerSubsystem` _asplayer_controller) "/Game/ShockerPTGC/Core/Engine/Controllers/IMC_Default.IMC_Default" 0 (struct)))

(event `EnhancedInput|/Game/ShockerPTGC/Core/Engine/Controllers/IA_Move`
  (params (ActionValue :type "Float (double-precision)") (ElapsedSeconds :type "Float (double-precision)") (TriggeredSeconds :type "Float (double-precision)") (InputAction :type "InputAction Object Reference" :default "/Game/ShockerPTGC/Core/Engine/Controllers/IA_Move.IA_Move"))
  (bind (_returnvalue_x _returnvalue_y _returnvalue_z) (`KismetMathLibrary.BreakVector` (`SceneComponent.K2_GetComponentLocation` (`self.Paddle`))))
  (:`Triggered`
    (`SceneComponent.K2_SetWorldLocation` (`self.Paddle`) (`KismetMathLibrary.MakeVector` (`KismetMathLibrary.FClamp` (+ (* ActionValue (`self.MovementScaler`)) _returnvalue_x) -1250.0 1250.0) _returnvalue_y _returnvalue_z) false false)))

(event `self.ReceiveBeginPlay`
  (bind _returnvalue (`|CreateWidget` "/Game/ShockerPTGC/Core/UI/Widgets/WBP_Pause.WBP_Pause_C"))
  (set `self.Pause Ref` _returnvalue))

(event `EnhancedInput|/Game/ShockerPTGC/Core/Engine/Controllers/IA_Pause`
  (params (ActionValue :type Boolean) (ElapsedSeconds :type "Float (double-precision)") (TriggeredSeconds :type "Float (double-precision)") (InputAction :type "InputAction Object Reference" :default "/Game/ShockerPTGC/Core/Engine/Controllers/IA_Pause.IA_Pause"))
  (bind _pause_ref (`self.Pause Ref`))
  (:`Started`
    (`/Engine/EditorBlueprintResources/StandardMacros.FlipFlop`
      (:`A`
        (`UserWidget.AddToViewport` _pause_ref 0)
        (`GameplayStatics.SetGamePaused` true))
      (:`B`
        (`Widget.RemoveFromParent` _pause_ref)
        (`GameplayStatics.SetGamePaused` false)))))

(fn `UserConstructionScript`)